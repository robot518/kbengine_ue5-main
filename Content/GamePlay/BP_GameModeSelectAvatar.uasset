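; Game mode for the avatar selection screen in a KBEngine-networked game.
; BeginPlay creates and shows the UI_SelectAvatar widget and enables the mouse cursor.
; KBEngine event handlers add avatars to the widget's list box, both from the requested avatar list and from avatar creation results.
; The space geometry mapping event enters the game world by opening the level named after the first slash in the resource path, and posts a loading message.
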(event EventBeginPlay
  ;[1 1 1] Show UI
  (bind _returnvalue (UserInterface|CreateWidget "/Game/HUD/UI_SelectAvatar.UI_SelectAvatar_C"))
  (UserInterface|Viewport|AddtoViewport _returnvalue 0)
  (Variables|Default|SetUIObj _returnvalue)
  ;[1 1 1] Show Mouse
  (Variables|/Script/Engine.PlayerController|SetbShowMouseCursor (Game|GetPlayerController 0) true))

(event EventTick
  (params (DeltaSeconds :type Float%20%28single-precision%29)))

(event EventOnCreateAvatarResult
  (params (pEventData :type KB%20Event%20Data%20Object%20Reference))
  ;[1 1 1] Add AvatarInfos To ListBox
  (bind _askbevent_data_on_create_avatar_result (Utilities|Casting|CastToKBEventData_onCreateAvatarResult pEventData))
  (Default|AddAvatartoListBox (Variables|Default|GetUIObj) (Variables|/Script/KBEnginePlugins.KBEventData_onCreateAvatarResult|GetavatarInfos _askbevent_data_on_create_avatar_result)))

(event EventAddSpaceGeometryMapping
  (params (pEventData :type KB%20Event%20Data%20Object%20Reference))
  ;[1 1 1] Open Level -> Enter the game world
  (bind _askbevent_data_add_space_geometry_mapping (Utilities|Casting|CastToKBEventData_addSpaceGeometryMapping pEventData))
  (Game|OpenLevel(byName) (Utilities|String|StringToName (.RightS (Utilities|String|Split (Variables|/Script/KBEnginePlugins.KBEventData_addSpaceGeometryMapping|GetspaceResPath _askbevent_data_add_space_geometry_mapping) "/"))))
  (Default|DEBUGMSG (Variables|Default|GetUIObj) "loading scene..."))

(event EventOnReqAvatarList
  (params (pEventData :type KB%20Event%20Data%20Object%20Reference))
  ;[1 1 1] Add AvatarInfos To ListBox
  (bind _askbevent_data_on_req_avatar_list (Utilities|Casting|CastToKBEventData_onReqAvatarList pEventData))
  (for _array_element (Variables|/Script/KBEnginePlugins.KBEventData_onReqAvatarList|Getavatars _askbevent_data_on_req_avatar_list)
    (Default|AddAvatartoListBox (Variables|Default|GetUIObj) _array_element)))

(fn ConstructionScript)