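; World game mode for a KBEngine client that shows the world UI and mouse cursor and reacts to server events.
; A space geometry mapping event opens the level named in its resource path.
; HP, max HP and name events find the entity by ID and update its UI_Entity widget, with names applied only to hover car entities.
; State events on the player character toggle the revive button.
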(event EventBeginPlay
  ;[1 1 1] Create the LoginUI
  (bind _returnvalue (UserInterface|CreateWidget "/Game/HUD/UI_World.UI_World_C"))
  (UserInterface|Viewport|AddtoViewport _returnvalue 0)
  (Variables|Default|SetUIObj _returnvalue)
  ;[1 1 1] Show Mouse
  (Variables|/Script/Engine.PlayerController|SetbShowMouseCursor (Game|GetPlayerController 0) true))

(event EventTick
  (params (DeltaSeconds :type Float%20%28single-precision%29)))

(event EventSetName
  (params (pEventData :type KB%20Event%20Data%20Object%20Reference))
  ;[1 1 1] Set Name
  (bind _askbevent_data_set_name (Utilities|Casting|CastToKBEventData_set_name pEventData))
  (bind _returnvalue (Class|GameModeWorld|FindHoverCarEntity (Variables|/Script/KBEnginePlugins.KBEventData_set_name|GetentityID _askbevent_data_set_name)))
  (bind _asbp_hover_car (Utilities|Casting|CastToBP_Hover_Car _returnvalue)
    (:then
      (bind _asui_entity (Utilities|Casting|CastToUI_Entity (UserInterface|GetUserWidgetObject (Variables|/Game/HoverCarSystem/Blueprints/BP_Hover_Car.BP_Hover_Car_C|GetWidget _asbp_hover_car))))
      (Rendering|Components|TextRender|SetText (Variables|/Game/Entity/UI/UI_Entity.UI_Entity_C|GetNameLabel _asui_entity) (Utilities|Text|ToText(String) (Variables|/Script/KBEnginePlugins.KBEventData_set_name|Getname _askbevent_data_set_name))))
    (:CastFailed
      (bind _asbp_hover_car_effects (Utilities|Casting|CastToBP_Hover_Car_Effects _returnvalue))
      (bind _asui_entity_2 (Utilities|Casting|CastToUI_Entity (UserInterface|GetUserWidgetObject (Variables|/Game/HoverCarSystem/Blueprints/BP_HoverPlayer_Car.BP_HoverPlayer_Car_C|GetWidget _asbp_hover_car_effects))))
      (Rendering|Components|TextRender|SetText (Variables|/Game/Entity/UI/UI_Entity.UI_Entity_C|GetNameLabel _asui_entity_2) (Utilities|Text|ToText(String) (Variables|/Script/KBEnginePlugins.KBEventData_set_name|Getname _askbevent_data_set_name))))))

(event EventSetState
  (params (pEventData :type KB%20Event%20Data%20Object%20Reference))
  (bind _uiobj (Variables|Default|GetUIObj))
  (bind _relivebtn (Variables|/Game/HUD/UI_World.UI_World_C|GetReliveBtn _uiobj))
  ;[1 1 1] Set Name
  (bind _askbevent_data_set_state (Utilities|Casting|CastToKBEventData_set_state pEventData))
  (bind _returnvalue (Class|GameModeWorld|FindGameEntity (Variables|/Script/KBEnginePlugins.KBEventData_set_state|GetentityID _askbevent_data_set_state)))
  (Utilities|Casting|CastToGameEntity_BP _returnvalue
    (:CastFailed
      (Utilities|Casting|CastToPlayerCharacter_BP _returnvalue)
      (if (== (Variables|/Script/KBEnginePlugins.KBEventData_set_state|Getstate _askbevent_data_set_state) 1)
        (Widget|SetVisibility _relivebtn "Visible")
        (else
          (Widget|SetVisibility _relivebtn "Hidden"))))))

(event EventAddSpaceGeometryMapping
  (params (pEventData :type KB%20Event%20Data%20Object%20Reference))
  ;[1 1 1] Open Level -> Enter the game world
  (bind _askbevent_data_add_space_geometry_mapping (Utilities|Casting|CastToKBEventData_addSpaceGeometryMapping pEventData))
  (Game|OpenLevel(byName) (Utilities|String|StringToName (.RightS (Utilities|String|Split (Variables|/Script/KBEnginePlugins.KBEventData_addSpaceGeometryMapping|GetspaceResPath _askbevent_data_add_space_geometry_mapping) "/")))))

(event EventOnAddSkill
  (params (pEventData :type KB%20Event%20Data%20Object%20Reference)))

(event EventSetHP
  (params (pEventData :type KB%20Event%20Data%20Object%20Reference))
  ;[1 1 1] Set HP_Max
  (bind _askbevent_data_set_hp (Utilities|Casting|CastToKBEventData_set_HP pEventData))
  (bind _returnvalue (Class|GameModeWorld|FindGameEntity (Variables|/Script/KBEnginePlugins.KBEventData_set_HP|GetentityID _askbevent_data_set_hp)))
  (bind _asgame_entity_bp (Utilities|Casting|CastToGameEntity_BP _returnvalue)
    (:then
      (bind _asui_entity (Utilities|Casting|CastToUI_Entity (UserInterface|GetUserWidgetObject (Variables|/Game/Entity/GameEntity_BP.GameEntity_BP_C|GetWidget _asgame_entity_bp))))
      (Variables|/Game/Entity/UI/UI_Entity.UI_Entity_C|SetHP _asui_entity (Variables|/Script/KBEnginePlugins.KBEventData_set_HP|GetHP _askbevent_data_set_hp))
      (Default|UpdateHPBar _asui_entity))
    (:CastFailed
      (bind _asplayer_character_bp (Utilities|Casting|CastToPlayerCharacter_BP _returnvalue))
      (bind _asui_entity_2 (Utilities|Casting|CastToUI_Entity (UserInterface|GetUserWidgetObject (Variables|/Game/Entity/PlayerCharacter_BP.PlayerCharacter_BP_C|GetWidget _asplayer_character_bp))))
      (Variables|/Game/Entity/UI/UI_Entity.UI_Entity_C|SetHP _asui_entity_2 (Variables|/Script/KBEnginePlugins.KBEventData_set_HP|GetHP _askbevent_data_set_hp))
      (Default|UpdateHPBar _asui_entity_2))))

(event EventSetHPMax
  (params (pEventData :type KB%20Event%20Data%20Object%20Reference))
  ;[1 1 1] Set HP_Max
  (bind _askbevent_data_set_hp_max (Utilities|Casting|CastToKBEventData_set_HP_Max pEventData))
  (bind _returnvalue (Class|GameModeWorld|FindGameEntity (Variables|/Script/KBEnginePlugins.KBEventData_set_HP_Max|GetentityID _askbevent_data_set_hp_max)))
  (bind _asgame_entity_bp (Utilities|Casting|CastToGameEntity_BP _returnvalue)
    (:then
      (bind _asui_entity (Utilities|Casting|CastToUI_Entity (UserInterface|GetUserWidgetObject (Variables|/Game/Entity/GameEntity_BP.GameEntity_BP_C|GetWidget _asgame_entity_bp))))
      (Variables|/Game/Entity/UI/UI_Entity.UI_Entity_C|SetHP_Max _asui_entity (Variables|/Script/KBEnginePlugins.KBEventData_set_HP_Max|GetHP_Max _askbevent_data_set_hp_max))
      (Default|UpdateHPBar _asui_entity))
    (:CastFailed
      (bind _asplayer_character_bp (Utilities|Casting|CastToPlayerCharacter_BP _returnvalue))
      (bind _asui_entity_2 (Utilities|Casting|CastToUI_Entity (UserInterface|GetUserWidgetObject (Variables|/Game/Entity/PlayerCharacter_BP.PlayerCharacter_BP_C|GetWidget _asplayer_character_bp))))
      (Variables|/Game/Entity/UI/UI_Entity.UI_Entity_C|SetHP_Max _asui_entity_2 (Variables|/Script/KBEnginePlugins.KBEventData_set_HP_Max|GetHP_Max _askbevent_data_set_hp_max))
      (Default|UpdateHPBar _asui_entity_2))))

(fn ConstructionScript)