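; Hover car Blueprint that drives jet particle effects from the car's inputs.
; Each tick, forward, boost, side boost and drift inputs mark jets as active, with side boost firing same-side pairs and drift firing diagonal pairs.
; A final pass over the emitter array built in the construction script activates marked jets, deactivates the rest, then clears the marks, so overlapping inputs combine cleanly.
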(event EventBeginPlay
  (|CallParentFunction) ; This node is disabled and will not be called.\nDrag off pins to build functionality.
)

(event Collision|EventActorBeginOverlap
  (params (OtherActor :type Actor%20Object%20Reference)))

(event EventTick
  (params (DeltaSeconds :type Float%20%28single-precision%29))
  (|CallParentFunction DeltaSeconds)
  ;[0.1686 1 0.4752] Controls the particle systems
  (|Update_Particle_Effects))

(fn ConstructionScript
  (|CallParentFunction)
  (Variables|Default|SetEmitter_Array (Utilities|Array|MakeArray (Variables|Default|GetJet_Accelerate) (Variables|Default|GetJet_Turbo) (Variables|Default|GetJet_FL) (Variables|Default|GetJet_FR) (Variables|Default|GetJet_RL) (Variables|Default|GetJet_RR))))